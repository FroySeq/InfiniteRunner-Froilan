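; BP_cat_GM is the game mode for what appears to be an endless-runner cat game, handling spawning, distance tracking and game over.
; On BeginPlay it creates the HUD and starts a looping timer that randomly spawns an obstacle or enemy at a fixed point.
; Tick accumulates distance at a constant assumed speed and updates the HUD.
; GameOver stops counting, shows the restart button and cursor, then pauses after a short delay.
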(event Custom|SpawnRandom
  (Game|SpawnActorfromClass (select (Math|Random|RandomBool) "/Game/Blueprint/BP_Obstacles.BP_Obstacles_C" "/Game/Blueprint/BP_Enemies.BP_Enemies_C") (Math|Transform|MakeTransform "1400.000000, 0,-400.000000") "Undefined" 0 0))

(event Custom|Game%20Over
  (Variables|Default|SetGame%20is%20Over true)
  (Default|ShowRestartButton (Variables|Default|GetGame%20HUD))
  (Variables|/Script/Engine.PlayerController|SetbShowMouseCursor (Game|GetPlayerController 0) true)
  (Utilities|FlowControl|Delay 0.75)
  (Game|SetGamePaused true))

(event EventBeginPlay
  (Variables|Default|SetGame%20is%20Over false)
  (bind _returnvalue (UserInterface|CreateWidget "/Game/Blueprint/BP_GameHUD.BP_GameHUD_C" (Game|GetPlayerController 0)))
  (bind _output_get (Variables|Default|SetGame%20HUD _returnvalue))
  (UserInterface|Viewport|AddtoViewport _output_get 0)
  (Utilities|Time|SetTimerbyEvent (delegate Custom|SpawnRandom) 0.75 true))

(event EventTick
  (params (DeltaSeconds :type Float%20%28single-precision%29))
  (if (not (Variables|Default|GetGame%20is%20Over))
    (bind _output_get (Variables|Default|SetTotal%20Distance (+ (Variables|Default|GetTotal%20Distance) (* DeltaSeconds 1.4e+03))))
    (Default|UpdateDistanceText (Variables|Default|GetGame%20HUD) (/ _output_get 1e+02))))

(fn ConstructionScript)